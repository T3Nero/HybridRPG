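; Base character Blueprint for a hybrid RPG that supports interactions between characters with HUD dialogue.
; Interact locks both the instigator and itself via StartInteraction, which stops movement, then shows dialogue through the HUD widget on the game mode cached at BeginPlay.
; StopInteracting unlocks only this character and hides the dialogue.
; The construction script disables shadow casting on the dialogue indicator.
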(event EventBeginPlay
  (bind _asgm_hybrid_rpg (Utilities|Casting|CastToGM_HybridRPG (Game|GetGameMode)))
  (Variables|Default|SetAs%20GM%20Hybrid%20RPG _asgm_hybrid_rpg))

(event Collision|EventActorBeginOverlap
  (params (OtherActor :type Actor%20Object%20Reference)))

(event EventTick
  (params (DeltaSeconds :type Float%20%28single-precision%29)))

(event EventInteract
  (params (Instigator :type BP%20Character%20Base%20Object%20Reference))
  (CallFunction|StartInteraction Instigator)
  (CallFunction|StartInteraction)
  (CallFunction|ShowDialogue))

(event EventStopInteracting
  (CallFunction|EndInteraction))

(fn ConstructionScript
  (Rendering|SetCastShadow (Variables|Default|GetDialogueIndicator) false))

(fn ShowDialogue
  (Default|ShowDialogue (Variables|/Game/Blueprints/GM_HybridRPG.GM_HybridRPG_C|GetWBPHUD (Variables|Default|GetAs%20GM%20Hybrid%20RPG)) self))

(fn StartInteraction
  (Variables|Default|SetInteractionLocked true)
  (Components|Movement|StopMovementImmediately (Variables|Character|GetCharacterMovement)))

(fn EndInteraction
  (Variables|Default|SetInteractionLocked false)
  (CallFunction|HideDialogue))

(fn HideDialogue
  (Default|HideDialogue (Variables|/Game/Blueprints/GM_HybridRPG.GM_HybridRPG_C|GetWBPHUD (Variables|Default|GetAs%20GM%20Hybrid%20RPG))))