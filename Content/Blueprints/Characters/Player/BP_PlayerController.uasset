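; Player controller for a hybrid RPG that turns Enhanced Input actions into movement, NPC interaction, weapon equipping and quitting.
; It caches the BP_Player pawn on BeginPlay and moves it along world axes unless interaction is locked.
; Interact messages the first overlapping character; during an interaction, it reveals the full HUD speech bubble text, or ends the interaction once revealed.
; Equip actions set the player's weapon type and equipped flag.
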(event Input|EnhancedActionEvents|EnhancedInputActionIA_Move
  (params (ActionValue :type Vector%202D%20Structure) (ElapsedSeconds :type Float%20%28double-precision%29) (TriggeredSeconds :type Float%20%28double-precision%29) (InputAction :type Input%20Action%20Object%20Reference :default "/Game/Input/Actions/IA_Move.IA_Move"))
  (bind (_x _y) (Math|Vector2D|BreakVector2D ActionValue))
  (if (not (Variables|/Game/Blueprints/Characters/BP_CharacterBase.BP_CharacterBase_C|GetInteractionLocked (Variables|Default|GetAs%20BP%20Player)))
    (Pawn|Input|AddMovementInput (Variables|Default|GetAs%20BP%20Player) "1.000000,0.000000,0.000000" _x false)
    (Pawn|Input|AddMovementInput (Variables|Default|GetAs%20BP%20Player) "0.000000,1.000000,0.000000" _y false)))

(event Input|EnhancedActionEvents|EnhancedInputActionIA_Exit
  (params (ActionValue :type Boolean) (ElapsedSeconds :type Float%20%28double-precision%29) (TriggeredSeconds :type Float%20%28double-precision%29) (InputAction :type Input%20Action%20Object%20Reference :default "/Game/Input/Actions/IA_Exit.IA_Exit"))
  (:Started
    (Game|QuitGame 0 "Quit" false)))

(event Input|EnhancedActionEvents|EnhancedInputActionIA_Interact
  (params (ActionValue :type Boolean) (ElapsedSeconds :type Float%20%28double-precision%29) (TriggeredSeconds :type Float%20%28double-precision%29) (InputAction :type Input%20Action%20Object%20Reference :default "/Game/Input/Actions/IA_Interact.IA_Interact"))
  (bind _as_bp_player (Variables|Default|GetAs%20BP%20Player))
  (bind _as_gm_hybrid_rpg (Variables|/Game/Blueprints/Characters/BP_CharacterBase.BP_CharacterBase_C|GetAs%20GM%20Hybrid%20RPG _as_bp_player))
  (bind _wbphud (Variables|/Game/Blueprints/GM_HybridRPG.GM_HybridRPG_C|GetWBPHUD _as_gm_hybrid_rpg))
  (bind _wbp_speechbubble (Variables|/Game/UI/WBP_HUD.WBP_HUD_C|GetWBP_SpeechBubble _wbphud))
  (:Started
    (if (Variables|/Game/Blueprints/Characters/BP_CharacterBase.BP_CharacterBase_C|GetInteractionLocked (Variables|Default|GetAs%20BP%20Player))
      (if (Default|FinishedRevealingText _wbp_speechbubble)
        (Default|EndInteraction (Variables|Default|GetAs%20BP%20Player))
        (Class|BPIInteract|StopInteracting(Message) (Variables|Default|GetLastInteractedActor))
        (else
          (Default|RevealFullMessage _wbp_speechbubble)))
      (else
        (bind _array_element (Utilities|Array|ForEachLoopwithBreak (Collision|GetOverlappingActors (Variables|/Game/Blueprints/Characters/Player/BP_Player.BP_Player_C|GetInteractCollider (Variables|Default|GetAs%20BP%20Player)) "/Game/Blueprints/Characters/BP_CharacterBase.BP_CharacterBase_C" :!class /Script/Engine.PrimitiveComponent) :!label _label)
          (:LoopBody
            (if (!= _array_element (Variables|Default|GetAs%20BP%20Player))
              (Class|BPIInteract|Interact(Message) _array_element (Variables|Default|GetAs%20BP%20Player))
              (Variables|Default|SetLastInteractedActor _array_element)
              (goto _label Break))))))))

(event Input|EnhancedActionEvents|EnhancedInputActionIA_EquipDual
  (params (ActionValue :type Boolean) (ElapsedSeconds :type Float%20%28double-precision%29) (TriggeredSeconds :type Float%20%28double-precision%29) (InputAction :type Input%20Action%20Object%20Reference :default "/Game/Input/Actions/IA_EquipDual.IA_EquipDual"))
  (bind _as_bp_player (Variables|Default|GetAs%20BP%20Player))
  (:Started
    (Variables|/Game/Blueprints/Characters/Player/BP_Player.BP_Player_C|SetIsWeaponEquipped _as_bp_player true)
    (Variables|/Game/Blueprints/Characters/Player/BP_Player.BP_Player_C|SetE_WeaponType _as_bp_player "NewEnumerator6")))

(event Input|EnhancedActionEvents|EnhancedInputActionIA_EquipTwoHand
  (params (ActionValue :type Boolean) (ElapsedSeconds :type Float%20%28double-precision%29) (TriggeredSeconds :type Float%20%28double-precision%29) (InputAction :type Input%20Action%20Object%20Reference :default "/Game/Input/Actions/IA_EquipTwoHand.IA_EquipTwoHand"))
  (bind _as_bp_player (Variables|Default|GetAs%20BP%20Player))
  (:Started
    (Variables|/Game/Blueprints/Characters/Player/BP_Player.BP_Player_C|SetIsWeaponEquipped _as_bp_player true)
    (Variables|/Game/Blueprints/Characters/Player/BP_Player.BP_Player_C|SetE_WeaponType _as_bp_player "NewEnumerator1")))

(event EventBeginPlay
  (Input|AddMappingContext (PlayerController|LocalPlayerSubsystems|GetEnhancedInputLocalPlayerSubsystem self) "/Game/Input/IMP_HybridRPG.IMP_HybridRPG" 0 "(bIgnoreAllPressedKeysUntilRelease=True,bForceImmediately=False,bNotifyUserSettings=False)")
  (bind _asbp_player (Utilities|Casting|CastToBP_Player (Game|GetPlayerCharacter 0)))
  (Variables|Default|SetAs%20BP%20Player _asbp_player))

(fn ConstructionScript)