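; BP_NPC is an interactable NPC that can wander at random and shows a dialogue indicator.
; When patrol is enabled, it loops AI moves to random navigable points within a radius of its current position, pausing for a random retriggerable delay whether a move succeeds or fails.
; Starting an interaction hides the indicator and blocks the next patrol move.
; Ending it restores the indicator and resumes patrol.
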(event Custom|PatrolRandomLocation
  (Utilities|FlowControl|RetriggerableDelay (Math|Random|RandomFloatinRange (Variables|Default|GetMinPatrolDelay) (Variables|Default|GetMaxPatrolDelay)))
  (if (not (Variables|Default|GetInteractionLocked))
    (bind _randomlocation (Class|NavigationSystemV1|GetRandomLocationinNavigableRadius (Transformation|GetActorLocation) (Variables|Default|GetPatrolRadius) 0 "/Script/AIModule.NavFilter_AIControllerDefault"))
    (AI|AIMoveTo self _randomlocation 0 5e+01 false
      (:OnSuccess
        _)
      (:OnFail
        _))
    (CallFunction|PatrolRandomLocation)))

(event EventBeginPlay
  (|CallParentFunction)
  (if (Variables|Default|GetCanPatrol)
    (bind _randomlocation (Class|NavigationSystemV1|GetRandomLocationinNavigableRadius (Transformation|GetActorLocation) (Variables|Default|GetPatrolRadius) 0 "/Script/AIModule.NavFilter_AIControllerDefault"))
    (AI|AIMoveTo self _randomlocation 0 5e+01 false
      (:OnSuccess
        _)
      (:OnFail
        _))
    (CallFunction|PatrolRandomLocation)))

(fn ConstructionScript
  (|CallParentFunction))

(fn StartInteraction
  (params (LookAtTarget :type Actor%20Object%20Reference))
  (|CallParentFunction LookAtTarget)
  (Rendering|SetVisibility (Variables|Default|GetDialogueIndicator) false false)
  (Variables|Default|SetInteractionLocked true))

(fn EndInteraction
  (|CallParentFunction)
  (Rendering|SetVisibility (Variables|Default|GetDialogueIndicator) true false)
  (Variables|Default|SetInteractionLocked false)
  (if (Variables|Default|GetCanPatrol)
    (CallFunction|PatrolRandomLocation)))